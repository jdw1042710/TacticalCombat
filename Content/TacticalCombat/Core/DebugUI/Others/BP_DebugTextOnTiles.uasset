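; Debug actor that labels walkable grid tiles with toggleable text: tile index and pathfinding enter cost, heuristic, start cost and sort order.
; On BeginPlay it finds BP_Grid and binds to its tile-data, destruction and pathfinding delegates.
; TextRenderActors are spawned on demand, cached by tile index, scaled to tile size and longest entry, and destroyed when unneeded.
; Changing the display flags refreshes all tiles or clears every label.
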(event `self.ReceiveBeginPlay`
  (bind _gridpathfinding (`Grid.GridPathfinding` (`self.Grid`)))
  (bind _returnvalue (`GameplayStatics.GetActorOfClass` "/Game/TacticalCombat/Core/Grid/BP_Grid.BP_Grid_C"))
  (bind _output_get (set `self.Grid` _returnvalue))
  (`/Engine/EditorBlueprintResources/StandardMacros.IsValid` _output_get
    (:`Is Valid`
      (add `Grid.OnTileDataUpdated` _output_get (`|CreateDelegate` :!event `UpdateTextOnTile`))
      (add `Grid.OnGridDestroyed` _output_get (`|CreateDelegate` :!event `ClearAllTextActors`))
      (add `GridPathfinding.OnPathfindingDataUpdated` _gridpathfinding (`|CreateDelegate` :!event `UpdateTextOnTile`))
      (add `GridPathfinding.OnPathfindingDataCleared` _gridpathfinding (`|CreateDelegate` :!event `UpdateTextOnAllTiles`)))))

(fn `CheckWantToDisplayAnyText`
  (returns (ReturnValue :type Boolean))
  (return (or (`self.bShowTileIndexes`) (`self.bShowCostToEnterTile`) (`self.bShowMinCostToTarget`) (`self.bShowCostFromStart`) (`self.bShowSortOrder`))))

(fn `ClearAllTextActors`
  (bind _values (`BlueprintMapLibrary.Map_Values` (`self.SpawnedTexts`)))
  (for _array_element _values
    (`self.K2_DestroyActor` _array_element))
  (`BlueprintMapLibrary.Map_Clear` (`self.SpawnedTexts`))
  (return))

(fn `DestoryTextActor`
  (params (Index :type "IntPoint Structure"))
  (locals (Actor :type "TextRenderActor Object Reference"))
  (bind _output_get (set `local.Actor` (`BlueprintMapLibrary.Map_Find` (`self.SpawnedTexts`) Index)))
  (`/Engine/EditorBlueprintResources/StandardMacros.IsValid` _output_get
    (:`Is Valid`
      (`self.K2_DestroyActor` _output_get)
      (`BlueprintMapLibrary.Map_Remove` (`self.SpawnedTexts`) (`local.Index`))
      (return))))

(fn `GetTextActor`
  (params (Index :type "IntPoint Structure"))
  (returns (TextRenderActor :type "TextRenderActor Object Reference"))
  (locals (Actor :type "TextRenderActor Object Reference"))
  (bind _actor (`local.Actor`))
  (bind _output_get (set `local.Actor` (`BlueprintMapLibrary.Map_Find` (`self.SpawnedTexts`) Index)))
  (`/Engine/EditorBlueprintResources/StandardMacros.IsValid` _output_get
    (:`Is Valid`
      (return (`local.Actor`)))
    (:`Is Not Valid`
      (bind _returnvalue (`|SpawnActorFromClass` "/Script/Engine.TextRenderActor" (`KismetMathLibrary.MakeTransform` (0.0 0.0 0.0)) "AlwaysSpawn" "OverrideRootScale" null null))
      (set `local.Actor` _returnvalue)
      (`BlueprintMapLibrary.Map_Add` (`self.SpawnedTexts`) (`local.Index`) (`local.Actor`))
      (`self.SetActorTickEnabled` _actor false)
      (`self.SetActorEnableCollision` _actor false)
      (return _actor))))

(fn `Set Show Tile Texts`
  (params (bShowTileIndexes :type Boolean) (bShowCostToEnterTile :type Boolean) (bShowMinCostToTarget :type Boolean) (bShowCostFromStart :type Boolean) (bShowSortOrder :type Boolean))
  (set `self.bShowTileIndexes` bShowTileIndexes)
  (set `self.bShowCostToEnterTile` bShowCostToEnterTile)
  (set `self.bShowMinCostToTarget` bShowMinCostToTarget)
  (set `self.bShowCostFromStart` bShowCostFromStart)
  (set `self.bShowSortOrder` bShowSortOrder)
  (`self.UpdateTextOnAllTiles`)
  (return))

(fn `UpdateTextOnAllTiles`
  (if (`self.CheckWantToDisplayAnyText`)
    (bind _returnvalue (`Grid.GetAllIndexesFromTileData` (`self.Grid`)))
    (for _array_element _returnvalue
      (`self.UpdateTextOnTile` _array_element))
    (else
      (`self.ClearAllTextActors`))))

(fn `UpdateTextOnTile`
  (params (Index :type "IntPoint Structure"))
  (locals (Data :type "TileData Structure") (`Text Actor` :type "TextRenderActor Object Reference") (Text :type "Array of String") (PathfindingData :type "PathfindingData Structure") (TextLengths :type "Array of Integer"))
  (bind (_index_x _index_y) (break `IntPoint` (`local.Index`)))
  (bind (_infinitevalue _index _costtoentertile _costfromstart _heuristicscosttotarget) (break `PathfindingData` (`local.PathfindingData`)))
  (bind (_infinitevalue_2 _index_2 _costtoentertile_2 _costfromstart_2) (break `PathfindingData` (`local.PathfindingData`)))
  (bind (_gridtilesize_x _gridtilesize_y) (`KismetMathLibrary.BreakVector` (`Grid.GridTileSize` (`self.Grid`))))
  (bind _textrender (`TextRenderActor.TextRender` (`local.Text Actor`)))
  (bind _returnvalue (`KismetStringLibrary.Concat_StrStr` (`KismetStringLibrary.Conv_IntToString` _index_x) ", " (`KismetStringLibrary.Conv_IntToString` _index_y)))
  (bind _returnvalue_2 (`KismetArrayLibrary.Array_Find` (`GridPathfinding.GetDiscoveredTiles` (`Grid.GridPathfinding` (`self.Grid`))) (`local.Index`)))
  (bind (_value _returnvalue_3) (`BlueprintMapLibrary.Map_Find` (`GridPathfinding.GetPathfindingData` (`Grid.GridPathfinding` (`self.Grid`))) (`local.Index`)))
  (bind _returnvalue_4 (`KismetStringLibrary.Concat_StrStr` "Enter: " (`KismetStringLibrary.Conv_IntToString` (`.CostToEnterTile` (break `PathfindingData` (`local.PathfindingData`))))))
  (bind _returnvalue_5 (`KismetStringLibrary.Concat_StrStr` "Heuristics: " (`KismetStringLibrary.Conv_IntToString` _heuristicscosttotarget)))
  (bind _returnvalue_6 (`KismetStringLibrary.Concat_StrStr` "Start: " (`KismetStringLibrary.Conv_IntToString` _costfromstart_2)))
  (bind _returnvalue_7 (`KismetStringLibrary.Concat_StrStr` "Sort Order: " (`KismetStringLibrary.Conv_IntToString` _returnvalue_2)))
  (if (`self.CheckWantToDisplayAnyText`)
    (bind (_data _returnvalue_8) (`Grid.GetTileDataFromIndex` (`self.Grid`) Index))
    (if _returnvalue_8
      (bind _output_get (set `local.Data` _data))
      (bind _returnvalue_9 (`TileDataUtility.IsTileWalkable` (`.Type` (break `TileData` _output_get))))
      (if _returnvalue_9
        (`|ExecutionSequence`
          (:`then_0`
            (`|ExecutionSequence`
              (:`then_0`
                (if (`self.bShowTileIndexes`)
                  (`KismetArrayLibrary.Array_Add` (`local.Text`) _returnvalue)
                  (`KismetArrayLibrary.Array_Add` (`local.TextLengths`) (`KismetStringLibrary.Len` _returnvalue))))
              (:`then_1`
                (if (or (`self.bShowCostToEnterTile`) (`self.bShowMinCostToTarget`) (`self.bShowCostFromStart`) (`self.bShowSortOrder`))
                  (if _returnvalue_3
                    (set `local.PathfindingData` _value)
                    (`|ExecutionSequence`
                      (:`then_0`
                        (if (`self.bShowCostToEnterTile`)
                          (`KismetArrayLibrary.Array_Add` (`local.Text`) _returnvalue_4)
                          (`KismetArrayLibrary.Array_Add` (`local.TextLengths`) (`KismetStringLibrary.Len` _returnvalue_4))))
                      (:`then_1`
                        (if (`self.bShowMinCostToTarget`)
                          (if (!= _infinitevalue _heuristicscosttotarget)
                            (`KismetArrayLibrary.Array_Add` (`local.Text`) _returnvalue_5)
                            (`KismetArrayLibrary.Array_Add` (`local.TextLengths`) (`KismetStringLibrary.Len` _returnvalue_5)))))
                      (:`then_2`
                        (if (`self.bShowCostFromStart`)
                          (if (!= _infinitevalue_2 _costfromstart_2)
                            (`KismetArrayLibrary.Array_Add` (`local.Text`) _returnvalue_6)
                            (`KismetArrayLibrary.Array_Add` (`local.TextLengths`) (`KismetStringLibrary.Len` _returnvalue_6)))))
                      (:`then_3`
                        (if (`self.bShowSortOrder`)
                          (if (!= _returnvalue_2 -1)
                            (`KismetArrayLibrary.Array_Add` (`local.Text`) _returnvalue_7)
                            (`KismetArrayLibrary.Array_Add` (`local.TextLengths`) (`KismetStringLibrary.Len` _returnvalue_7)))))))))))
          (:`then_1`
            (if (> (`KismetArrayLibrary.Array_Length` (`local.Text`)) 0)
              (bind _textrenderactor (`self.GetTextActor` (`local.Index`)))
              (set `local.Text Actor` _textrenderactor)
              (`TextRenderComponent.K2_SetText` _textrender (`KismetTextLibrary.Conv_StringToText` (`KismetStringLibrary.JoinStringArray` (`local.Text`) " \n")))
              (`TextRenderComponent.SetHorizontalAlignment` _textrender "EHTA_Center")
              (`TextRenderComponent.SetVerticalAlignment` _textrender "EVRTA_TextCenter")
              (`self.K2_SetActorTransform` (`local.Text Actor`) (`KismetMathLibrary.MakeTransform` (+ (.location (`.Transform` (break `TileData` (`local.Data`)))) (0.0 0.0 1.0)) (struct :`Pitch` 90.0 :`Yaw` 180.0) (`KismetMathLibrary.Conv_DoubleToVector` (/ _gridtilesize_y (`KismetMathLibrary.Conv_IntToDouble` (* (`.MaxValue` (`KismetMathLibrary.MaxOfIntArray` (`local.TextLengths`))) 25))))) false false)
              (return)
              (else
                (`self.DestoryTextActor` (`local.Index`))))))
        (else
          (`self.DestoryTextActor` (`local.Index`) :!label _label)
          (return)))
      (else
        (goto _label)))))

(fn `UserConstructionScript`)